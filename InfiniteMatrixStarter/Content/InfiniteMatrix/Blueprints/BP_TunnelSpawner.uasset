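; Spawner actor that builds the chained tunnel segments of the level and populates them with enemies and health packs.
; On BeginPlay it destroys existing tunnels, pickups and enemies, then spawns a short starting run from the player's location.
; Each new tunnel attaches at the previous one's SpawnPoint, randomizes its wall and stores a reference back to the spawner.
; Each spawn also rolls separately for a health pack and an enemy at randomized offsets.
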(event `self.ReceiveBeginPlay`
  (`self.SpawnInitialTunnels`))

(fn `Spawn Tunnel`
  (params (`Spawn Location` :type "Vector Structure"))
  (locals (NewLocalVar :type "/Game/InfiniteMatrix/Blueprints/BP_Tunnel Object Reference"))
  (`|ExecutionSequence`
    (:`then_0`
      (bind _returnvalue (`|SpawnActorFromClass` "/Game/InfiniteMatrix/Blueprints/BP_Tunnel.BP_Tunnel_C" (`KismetMathLibrary.MakeTransform` `Spawn Location`) "Undefined" "MultiplyWithRoot" null null))
      (bind _output_get (set `self.Newest Tunnel` _returnvalue))
      (set `/Game/InfiniteMatrix/Blueprints/BP_Tunnel.TunnelSpawner` self _output_get)
      (`/Game/InfiniteMatrix/Blueprints/BP_Tunnel.RandomizeWall` _output_get))
    (:`then_1`
      (`self.SpawnHealthPack`))
    (:`then_2`
      (`self.SpawnEnemy`))))

(fn `SpawnEnemy`
  (bind _returnvalue (`KismetMathLibrary.RandomFloatInRange` -400.0 400.0))
  (bind (_returnvalue_x _returnvalue_y _returnvalue_z) (`KismetMathLibrary.BreakVector` (`self.K2_GetActorLocation` (`self.Newest Tunnel`))))
  (if (< (`KismetMathLibrary.RandomIntegerInRange` 0 10) 8)
    (`|SpawnActorFromClass` "/Game/InfiniteMatrix/Blueprints/BP_Enemy.BP_Enemy_C" (`KismetMathLibrary.MakeTransform` (`KismetMathLibrary.MakeVector` (+ _returnvalue_x 1500.0) (+ _returnvalue_y _returnvalue) (+ _returnvalue_z _returnvalue))) "AdjustIfPossibleButDontSpawnIfColliding" "MultiplyWithRoot" null null)))

(fn `SpawnHealthPack`
  (bind _returnvalue (`KismetMathLibrary.RandomFloatInRange` -400.0 400.0))
  (bind (_returnvalue_x _returnvalue_y _returnvalue_z) (`KismetMathLibrary.BreakVector` (`self.K2_GetActorLocation` (`self.Newest Tunnel`))))
  (if (< (`KismetMathLibrary.RandomIntegerInRange` 0 10) 8)
    (`|SpawnActorFromClass` "/Game/InfiniteMatrix/Blueprints/BP_HealthPack.BP_HealthPack_C" (`KismetMathLibrary.MakeTransform` (`KismetMathLibrary.MakeVector` (+ _returnvalue_x 1000.0) (+ _returnvalue_y _returnvalue) (+ _returnvalue_z _returnvalue))) "AdjustIfPossibleButDontSpawnIfColliding" "MultiplyWithRoot" null null)))

(fn `SpawnInitialTunnels`
  (`|ExecutionSequence`
    (:`then_0`
      (bind _outactors (`GameplayStatics.GetAllActorsOfClass` "/Game/InfiniteMatrix/Blueprints/BP_HealthPack.BP_HealthPack_C"))
      (for _array_element _outactors
        (`self.K2_DestroyActor` _array_element)))
    (:`then_1`
      (bind _outactors_2 (`GameplayStatics.GetAllActorsOfClass` "/Game/InfiniteMatrix/Blueprints/BP_Tunnel.BP_Tunnel_C"))
      (for _array_element_2 _outactors_2
        (`self.K2_DestroyActor` _array_element_2)))
    (:`then_2`
      (bind _outactors_3 (`GameplayStatics.GetAllActorsOfClass` "/Game/InfiniteMatrix/Blueprints/BP_Enemy.BP_Enemy_C"))
      (for _array_element_3 _outactors_3
        (`self.K2_DestroyActor` _array_element_3)))
    (:`then_3`
      (for _ (range 3)
        (`/Engine/EditorBlueprintResources/StandardMacros.IsValid` (`self.Newest Tunnel`)
          (:`Is Valid`
            (`self.SpawnTunnelAtSpawnPoint`))
          (:`Is Not Valid`
            (`self.Spawn Tunnel` (`self.K2_GetActorLocation` (`GameplayStatics.GetPlayerPawn` 0)))))))))

(fn `SpawnTunnelAtSpawnPoint`
  (`self.Spawn Tunnel` (`SceneComponent.K2_GetComponentLocation` (`/Game/InfiniteMatrix/Blueprints/BP_Tunnel.SpawnPoint` (`self.Newest Tunnel`)))))

(fn `UserConstructionScript`)