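; BP_Enemy is an enemy actor that awards or costs the player score and destroys itself on contact.
; A projectile hit on ProjectileHitBox adds HitScore to the firing player and destroys both actors; a player hit there removes only that box.
; A player hit on PlayerCollideBox deducts score and health, prints a debug string and destroys the enemy.
; The enemy also destroys itself when the player leaves PassBox.
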(event `self.ProjectileHitBox.OnComponentHit`
  (params (HitComponent :type "PrimitiveComponent Object Reference") (OtherActor :type "Actor Object Reference") (OtherComp :type "PrimitiveComponent Object Reference") (NormalImpulse :type "Vector Structure") (Hit :type "HitResult Structure (by ref)"))
  (`|ExecutionSequence`
    (:`then_0`
      (cast `/Game/InfiniteMatrix/Blueprints/BP_Player` OtherActor)
      (`ActorComponent.K2_DestroyComponent` (`self.ProjectileHitBox`)))
    (:`then_1`
      (bind _asbp_projectile (cast `/Game/InfiniteMatrix/Blueprints/BP_Projectile` OtherActor))
      (`/Game/InfiniteMatrix/Blueprints/BP_Player.UpdateScore` (`/Game/InfiniteMatrix/Blueprints/BP_Projectile.ParentPlayer` _asbp_projectile) (`self.HitScore`))
      (`self.K2_DestroyActor` _asbp_projectile)
      (`self.K2_DestroyActor` :!label _label))))

(event `self.PlayerCollideBox.OnComponentHit`
  (params (HitComponent :type "PrimitiveComponent Object Reference") (OtherActor :type "Actor Object Reference") (OtherComp :type "PrimitiveComponent Object Reference") (NormalImpulse :type "Vector Structure") (Hit :type "HitResult Structure (by ref)"))
  (bind _asbp_player (cast `/Game/InfiniteMatrix/Blueprints/BP_Player` OtherActor))
  (`/Game/InfiniteMatrix/Blueprints/BP_Player.UpdateScore` _asbp_player (* (`self.HitScore`) -1))
  (set `/Game/InfiniteMatrix/Blueprints/BP_Player.Health` (- (`/Game/InfiniteMatrix/Blueprints/BP_Player.Health` _asbp_player) (`self.HealthLose`)) _asbp_player)
  (`KismetSystemLibrary.PrintString` "Hello")
  (goto _label))

(event `self.PassBox.OnComponentEndOverlap`
  (params (OverlappedComponent :type "PrimitiveComponent Object Reference") (OtherActor :type "Actor Object Reference") (OtherComp :type "PrimitiveComponent Object Reference") (OtherBodyIndex :type Integer))
  (cast `/Game/InfiniteMatrix/Blueprints/BP_Player` OtherActor)
  (`self.K2_DestroyActor`))

(fn `UserConstructionScript`)